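; BP_OrbitActor is an actor that moves its Cube component in a continuous orbit around the actor's origin.
; Each Tick advances an angle in degrees by delta time times OrbitSpeed.
; Cosine and sine of that angle, scaled by OrbitRadius, set the cube's relative X and Y, while sine scaled by Inclination sets Z to tilt the orbit.
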(event `self.ReceiveTick`
  (params (DeltaSeconds :type "Float (single-precision)"))
  (bind _orbitradius_ (`self.OrbitRadius `))
  (bind _output_get (set `self.CurrentTime ` (+ (`self.CurrentTime `) (* DeltaSeconds (`self.OrbitSpeed `)))))
  (bind _returnvalue (`KismetMathLibrary.DegreesToRadians` _output_get))
  (bind _returnvalue_2 (`KismetMathLibrary.Sin` _returnvalue))
  (`SceneComponent.K2_SetRelativeLocation` (`self.Cube`) (`KismetMathLibrary.MakeVector` (* (`KismetMathLibrary.Cos` _returnvalue) _orbitradius_) (* _orbitradius_ _returnvalue_2) (* (`self.Inclination `) _returnvalue_2)) false false))

(fn `UserConstructionScript`)