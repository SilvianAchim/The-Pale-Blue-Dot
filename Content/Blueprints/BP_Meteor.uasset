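; BP_Meteor is an actor meant to orbit BP_Earth, repositioning itself every Tick.
; It looks up the Earth actor and offsets from its location using sine and cosine of an angle, scaled by orbit radius and inclination.
; The angle derives only from the current frame's delta time and speed, so it does not accumulate.
; Inclination is converted to radians in place every Tick, shrinking it toward zero.
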(event `self.ReceiveBeginPlay`)

(event `self.ReceiveTick`
  (params (DeltaSeconds :type "Float (single-precision)"))
  (set `self.CurrentAngle` (`KismetMathLibrary.DegreesToRadians` (mod (+ (* DeltaSeconds (`self.OrbitSpeed`)) 0.0) 360.0)))
  (set `self.OrbitInclination ` (`KismetMathLibrary.DegreesToRadians` (`self.OrbitInclination `)))
  (bind _returnvalue (`GameplayStatics.GetActorOfClass` "/Game/Blueprints/BP_Earth.BP_Earth_C"))
  (bind (_returnvalue_x _returnvalue_y _returnvalue_z) (`KismetMathLibrary.BreakVector` (`self.K2_GetActorLocation` _returnvalue)))
  (`self.K2_SetActorLocation` (`KismetMathLibrary.MakeVector` (+ _returnvalue_x (* (* (`self.OrbitRadius`) (`KismetMathLibrary.Cos` (`self.CurrentAngle`))) (`KismetMathLibrary.Cos` (`self.OrbitInclination `)))) (+ _returnvalue_y (* (* (`self.OrbitRadius`) (`KismetMathLibrary.Sin` (`self.CurrentAngle`))) (`KismetMathLibrary.Sin` (`self.OrbitInclination `)))) (+ _returnvalue_z (* (`self.OrbitRadius`) (`KismetMathLibrary.Sin` (`self.OrbitInclination `)))))))

(fn `UserConstructionScript`)