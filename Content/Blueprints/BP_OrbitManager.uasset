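; BP_OrbitManager drives a meteor along an orbit, along with a third-person and a first-person camera.
; Each tick it advances orbit time, moves the meteor to that orbit point and interpolates its roll toward the target.
; The third-person camera follows the orbit with time and radius offsets, smoothly turning toward the meteor, while the first-person camera faces the world origin.
; Input functions adjust target roll and clamped orbit inclination.
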(event `self.ReceiveTick`
  (params (DeltaSeconds :type "Float (single-precision)"))
  (`self.Update Current Time` DeltaSeconds)
  ;[0.3278 0.2542 0.4072] Update Meteor location
  (bind _newparam (`self.Get Orbit Location` (`self.Current Time `) (`self.Orbit Radius`)))
  (`self.Update Actor Location` _newparam DeltaSeconds (`self.Meteor`))
  (`self.Update Meteor Roll` DeltaSeconds)
  (`self.Update Third Person Camera` DeltaSeconds)
  (`self.Update First Person Camera`))

(fn `Update First Person Camera`
  (`self.K2_SetActorRotation` (`self.First Person Camera`) (`KismetMathLibrary.FindLookAtRotation` (`self.K2_GetActorLocation` (`self.First Person Camera`)) (0.0 0.0 0.0)) false))

(fn `Update Meteor Roll`
  (params (`Delta Seconds` :type "Float (double-precision)"))
  (bind _targeted_rotation_roll (`KismetMathLibrary.BreakRotator` (`self.Targeted Rotation`)))
  (bind _output_get (set `self.Targeted Rotation` (`KismetMathLibrary.MakeRotator` (mod _targeted_rotation_roll 360.0))))
  (`self.K2_SetActorRotation` (`self.Meteor`) (`KismetMathLibrary.RInterpTo` (`self.K2_GetActorRotation` (`self.Meteor`)) _output_get `Delta Seconds` (`self. Interp Speed`)) false))

(fn `Update Pitch`
  (params (Value :type "Float (double-precision)"))
  ;[0.3278 0.2542 0.4072] Increment Inclination on user input
  (set `self.Orbit Inclination ` (`KismetMathLibrary.FClamp` (+ Value (`self.Orbit Inclination `)) 0.0 180.0)))

(fn `Update Roll`
  (params (Value :type "Float (double-precision)"))
  (bind (_targeted_rotation_roll _targeted_rotation_pitch _targeted_rotation_yaw) (`KismetMathLibrary.BreakRotator` (`self.Targeted Rotation`)))
  ;[0.8036 0.6267 1 0.7] Change the roll (x-axis) on user input
  (set `self.Targeted Rotation` (`KismetMathLibrary.MakeRotator` (`KismetMathLibrary.FClamp` (+ _targeted_rotation_roll (* Value (`self.Rotation Speed`))) -360.0 360.0) _targeted_rotation_pitch _targeted_rotation_yaw)))

(fn `Update Third Person Camera`
  (params (`Delta Seconds` :type "Float (double-precision)"))
  ;[0.3278 0.2542 0.4072 0.7] Update camera location
  (bind _newparam (`self.Get Orbit Location` (+ (`self.Current Time `) (`self.Third Person Camera Time Offset`)) (+ (`self.Orbit Radius`) (`self.Third Person Camera Radius Offset`))))
  (`self.Update Actor Location` _newparam `Delta Seconds` (`self.Third Person Camera`))
  ;[0.3278 0.2542 0.4072 0.7] Update Camera Rotation
  (`self.K2_SetActorRotation` (`self.Third Person Camera`) (`KismetMathLibrary.RInterpTo` (`self.K2_GetActorRotation` (`self.Third Person Camera`)) (`KismetMathLibrary.FindLookAtRotation` (`self.K2_GetActorLocation` (`self.Third Person Camera`)) (`self.K2_GetActorLocation` (`self.Meteor`))) `Delta Seconds` 4.0) false))

(fn `UserConstructionScript`)