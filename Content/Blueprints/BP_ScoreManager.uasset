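; BP_ScoreManager saves and reads back a persistent history of player scores from the "Score" save slot.
; SaveScore appends BP_EarthMoonSystem's completed-orbit count, stamped with the current date, to the SaveGame_SaveUserScore list.
; When that save fails to load, it creates a new one with a blank entry, so that run's score is not recorded.
; GetScoreList returns the stored list for other Blueprints.
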(fn `Get Score List`
  (returns (ScoreList :type "Array of /Game/Blueprints/Struct_UserScore Structure"))
  (bind _returnvalue (`GameplayStatics.LoadGameFromSlot` "Score"))
  (bind _assave_game_save_user_score (cast `/Game/Blueprints/SaveGame_SaveUserScore` _returnvalue))
  (return (`/Game/Blueprints/SaveGame_SaveUserScore.ScoreList` _assave_game_save_user_score)))

(fn `Save Score`
  (bind _returnvalue (`GameplayStatics.GetActorOfClass` "/Game/Blueprints/BP_EarthMoonSystem.BP_EarthMoonSystem_C"))
  (bind _returnvalue_2 (`GameplayStatics.LoadGameFromSlot` "Score"))
  (bind _assave_game_save_user_score (cast `/Game/Blueprints/SaveGame_SaveUserScore` _returnvalue_2)
    (:`then`
      (`KismetArrayLibrary.Array_Add` (`/Game/Blueprints/SaveGame_SaveUserScore.ScoreList` _assave_game_save_user_score) (make `/Game/Blueprints/Struct_UserScore` (`/Game/Blueprints/BP_EarthMoonSystem.Orbits Completed` _returnvalue) (`KismetTextLibrary.Conv_TextToString` (`KismetTextLibrary.AsDate_DateTime` (`KismetMathLibrary.Now`)))))
      (`GameplayStatics.SaveGameToSlot` _assave_game_save_user_score "Score"))
    (:`CastFailed`
      (bind _returnvalue_3 (`GameplayStatics.CreateSaveGameObject` "/Game/Blueprints/SaveGame_SaveUserScore.SaveGame_SaveUserScore_C"))
      (`KismetArrayLibrary.Array_Add` (`/Game/Blueprints/SaveGame_SaveUserScore.ScoreList` _returnvalue_3))
      (`GameplayStatics.SaveGameToSlot` _returnvalue_3 "Score"))))

(fn `UserConstructionScript`)