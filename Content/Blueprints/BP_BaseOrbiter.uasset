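; Base orbiter Blueprint that moves a referenced Meteor actor along an inclined circular orbit around the world origin.
; While orbiting, Tick advances an angle in degrees by OrbitSpeed and converts it to a position using OrbitRadius and OrbitInclination.
; The Meteor eases toward that position with VInterpTo, without sweeping.
; StopOrResumeOrbit toggles the motion on and off.
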(event `self.ReceiveTick`
  (params (DeltaSeconds :type "Float (single-precision)"))
  (if (`self.Is Orbiting`)
    (`self.Update Current Time` DeltaSeconds)
    ;[0.3278 0.2542 0.4072] Update Meteor location
    (bind _new_location (`self.Get Orbit Location` (`self.Current Time `) (`self.Orbit Radius`)))
    (`self.Update Actor Location` _new_location DeltaSeconds (`self.Meteor`))))

(fn `Get Orbit Location`
  (params (Time :type "Float (double-precision)") (`Orbit Radius` :type "Float (double-precision)") (`Orbit Center` :type "Vector Structure"))
  (returns (`New Location` :type "Vector Structure"))
  (bind _returnvalue (`KismetMathLibrary.DegreesToRadians` Time))
  (bind _returnvalue_2 (`KismetMathLibrary.DegreesToRadians` (`self.Orbit Inclination `)))
  (return (+ (`KismetMathLibrary.MakeVector` (* (`KismetMathLibrary.Cos` _returnvalue) `Orbit Radius`) (* (* `Orbit Radius` (`KismetMathLibrary.Sin` _returnvalue)) (`KismetMathLibrary.Cos` _returnvalue_2)) (* (* `Orbit Radius` (`KismetMathLibrary.Sin` _returnvalue)) (`KismetMathLibrary.Sin` _returnvalue_2))) `Orbit Center`)))

(fn `Stop or Resume Orbit`
  (set `self.Is Orbiting` (not (`self.Is Orbiting`))))

(fn `Update Actor Location`
  (params (`New Location` :type "Vector Structure") (`Delta Seconds` :type "Float (double-precision)") (Actor :type "Actor Object Reference"))
  (`self.K2_SetActorLocation` Actor (`KismetMathLibrary.VInterpTo` (`self.K2_GetActorLocation` Actor) `New Location` `Delta Seconds` (`self. Interp Speed`)) false false))

(fn `Update Current Time`
  (params (DeltaTime :type "Float (double-precision)"))
  (set `self.Current Time ` (+ (`self.Current Time `) (* DeltaTime (`self.Orbit Speed`))))
  (return))

(fn `UserConstructionScript`)