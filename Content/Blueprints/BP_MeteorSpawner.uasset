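; Spawner actor that populates an orbital field of BP_Meteorit meteors when play begins.
; SpawnMeteors loops over the InitialMeteors count, spawning each meteor at a random distant X position and attaching it to a new scene component added on SpawnParent.
; It then randomizes each meteor's orbit radius, inclination, speed and starting time, and sets its Meteor reference to itself.
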(event `self.ReceiveBeginPlay`
  (`self.Spawn Meteors` (`self.Initial Meteors`)))

(fn `Spawn Meteors`
  (params (Count :type Integer))
  (bind _returnvalue (`KismetMathLibrary.RandomFloatInRange` 18000000.0 38000000.0))
  (for _ (range (+ Count 1))
    (bind _returnvalue_2 (`|SpawnActorFromClass` "/Game/Blueprints/BP_Meteorit.BP_Meteorit_C" (`KismetMathLibrary.MakeTransform` (`KismetMathLibrary.MakeVector` _returnvalue)) "Undefined" "MultiplyWithRoot" null null null))
    (bind _returnvalue_3 (`AddComponent|NODE_AddSceneComponent-0` :`self` (`self.Spawn Parent`)))
    (`self.K2_AttachToComponent` _returnvalue_2 _returnvalue_3 "None" "KeepRelative" "KeepRelative" "KeepRelative" true)
    (set `/Game/Blueprints/BP_BaseOrbiter.Orbit Radius` _returnvalue _returnvalue_2)
    (set `/Game/Blueprints/BP_BaseOrbiter.Orbit Inclination ` (`KismetMathLibrary.RandomFloatInRange` 0.0 180.0) _returnvalue_2)
    (set `/Game/Blueprints/BP_BaseOrbiter.Orbit Speed` (`KismetMathLibrary.RandomFloatInRange` 5.0 10.0) _returnvalue_2)
    (set `/Game/Blueprints/BP_BaseOrbiter.Current Time ` (`KismetMathLibrary.RandomFloatInRange` 0.0 360.0) _returnvalue_2)
    (set `/Game/Blueprints/BP_BaseOrbiter.Meteor` _returnvalue_2 _returnvalue_2)))

(fn `UserConstructionScript`)