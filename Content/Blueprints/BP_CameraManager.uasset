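; Camera manager actor that switches the first player's view between a first-person and a third-person camera.
; On BeginPlay it sets the view target of player controller 0 to the third-person camera.
; ChangeCamera uses a FlipFlop to alternate on each call, going to first person first, then back to third person.
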(event `self.ReceiveBeginPlay`
  (`PlayerController.SetViewTargetWithBlend` (`GameplayStatics.GetPlayerController` 0) (`self.Third Person Camera`) 0.0 "VTBlend_Linear" 0.0 false))

(fn `Change Camera`
  (`/Engine/EditorBlueprintResources/StandardMacros.FlipFlop`
    (:`A`
      (`PlayerController.SetViewTargetWithBlend` (`GameplayStatics.GetPlayerController` 0) (`self.First Person Camera`) 0.0 "VTBlend_Linear" 0.0 false))
    (:`B`
      (`PlayerController.SetViewTargetWithBlend` (`GameplayStatics.GetPlayerController` 0) (`self.Third Person Camera`) 0.0 "VTBlend_Linear" 0.0 false))))

(fn `UserConstructionScript`)