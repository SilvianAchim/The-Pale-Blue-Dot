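; Earth-Moon system actor that counts orbits of its referenced Meteor actor and triggers meteor showers.
; After the parent Tick, it captures the Meteor's location while the stored start is zero, then checks for proximity to it using a very large tolerance.
; A flag limits counting to once per entry into that zone, including the initial one.
; Every second count tells BP_MeteorSpawner to spawn a batch of meteors.
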(event `self.ReceiveTick`
  (params (DeltaSeconds :type "Float (single-precision)"))
  (`parent.ReceiveTick` DeltaSeconds)
  (`self.Set Initial Location`)
  (`self.Check Orbit`))

(fn `Check Orbit`
  (if (== (`self.K2_GetActorLocation` (`self.Meteor`)) (`self.Initial Orbit Location`) :`ErrorTolerance` 1698418540.401771)
    (if (not (`self.Has Completed Orbit`))
      (`self.Increment Orbit Count`)
      (set `self.Has Completed Orbit` true))
    (else
      (set `self.Has Completed Orbit` false))))

(fn `Increment Orbit Count`
  (bind _output_get (set `self.Orbits Completed` (+ (`self.Orbits Completed`) 1)))
  (if (== (mod _output_get 2) 0)
    (bind _returnvalue (`GameplayStatics.GetActorOfClass` "/Game/Blueprints/BP_MeteorSpawner.BP_MeteorSpawner_C"))
    (`/Game/Blueprints/BP_MeteorSpawner.Spawn Meteors` _returnvalue 20)))

(fn `Set Initial Location`
  (if (== (`self.Initial Orbit Location`) (0.0 0.0 0.0))
    (set `self.Initial Orbit Location` (`self.K2_GetActorLocation` (`self.Meteor`)))))

(fn `UserConstructionScript`)